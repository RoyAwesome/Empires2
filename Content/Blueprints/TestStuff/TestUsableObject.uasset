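; TestUsableObject is a test Blueprint for an interactable object that prints debug messages when use starts and stops.
; On hover, it creates a UseTest prompt widget for the User, cast to PlayerController, and adds it to the viewport.
; The widget reference is cached in ShowUseObject, so later prompt and hide events only toggle its visibility.
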(event `self.BTOnUsed`
  (params (User :type "Controller Object Reference"))
  ;[1 1 1] When the object is used, display a string
  (`KismetSystemLibrary.PrintString` "Object Used!"))

(event `self.BTStopUsed`
  (params (User :type "Controller Object Reference"))
  ;[1 1 1] When the object is done being used
  (`KismetSystemLibrary.PrintString` "Object done being used!"))

(event `self.BTHidePrompt`
  (bind _showuseobject (`self.ShowUseObject`))
  ;[1 1 1] Hide "Press E to use" when we are done with this object
  (`/Engine/EditorBlueprintResources/StandardMacros.IsValid` _showuseobject
    (:`Is Valid`
      (`Widget.SetVisibility` _showuseobject "Hidden"))))

(event `self.BTDisplayPrompt`
  (params (User :type "Controller Object Reference"))
  ;[1 1 1] Show the 'Press E to use' widget when we hover over the object.
  (`/Engine/EditorBlueprintResources/StandardMacros.IsValid` (`self.ShowUseObject`)
    (:`Is Valid`
      (`Widget.SetVisibility` (`self.ShowUseObject`) "Visible"))
    (:`Is Not Valid`
      (bind _asplayer_controller (cast `PlayerController` User))
      (bind _returnvalue (`|CreateWidget` "/Game/Blueprints/TestStuff/UseTest.UseTest_C" _asplayer_controller))
      (`UserWidget.AddToViewport` _returnvalue)
      (set `self.ShowUseObject` _returnvalue))))

(fn `UserConstructionScript`)