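; Player HUD Blueprint that manages the infantry HUD and the death, team, class and spawn screens.
; Open events lazily create and cache each widget, then toggle cursor and input mode; reopening the spawn screen refreshes its classes.
; BeginPlay opens the HUD, death opens the death screen, and spawning swaps back.
; Hit and damage notifications only print strings, and separate death-screen helper functions go uncalled here.
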(event `ShowCursor`
  (params (Focus :type "UserWidget Object Reference"))
  (bind _returnvalue (`self.GetOwningPlayerController`))
  ;[1 1 1] Hide/Show Cursor
  (set `PlayerController.bShowMouseCursor` true _returnvalue)
  (`WidgetBlueprintLibrary.SetInputMode_GameAndUIEx` _returnvalue Focus true))

(event `self.ReceiveBeginPlay`
  ;[1 1 1] When the Hud starts, Create the widgets we need
  (`self.OpenHUD`))

(event `HideCursor`
  (bind _returnvalue (`self.GetOwningPlayerController`))
  ;[1 1 1] Hide/Show Cursor
  (set `PlayerController.bShowMouseCursor` false _returnvalue)
  (`WidgetBlueprintLibrary.SetInputMode_GameOnly` _returnvalue))

(event `self.NotifyTookDamage`
  (params (FromWhere :type "Object.Vector Structure") (HowMuch :type Integer) (FromWho :type "PlayerState Object Reference"))
  (`KismetSystemLibrary.PrintString` "Took Damage"))

(event `OpenHUD`
  ;[1 1 1] Open/Close HUD
  (`/Engine/EditorBlueprintResources/StandardMacros.IsValid` (`self.HudWidget`)
    (:`Is Valid`
      _)
    (:`Is Not Valid`
      (bind _returnvalue (`|CreateWidget` "/Game/UI/InfantryHUD/InfantryHud.InfantryHud_C" (`self.GetOwningPlayerController`)))
      (bind _output_get (set `self.HudWidget` _returnvalue))))
  (`UserWidget.AddToViewport` _output_get 0)
  (`self.HideCursor`))

(event `self.NotifyLandedHit`
  (params (HitWhat :type "Pawn Object Reference"))
  (`KismetSystemLibrary.PrintString` "Hit Someone"))

(event `CloseHUD`
  ;[1 1 1] Open/Close HUD
  (`Widget.RemoveFromParent` (`self.HudWidget`)))

(event `self.NotifyDied`
  (params (Killer :type "PlayerState Object Reference"))
  (`self.OpenDeathScreen`))

(event `OpenDeathScreen`
  ;[1 1 1] Open/Close Death Screen
  (`/Engine/EditorBlueprintResources/StandardMacros.IsValid` (`self.DeathScreen`)
    (:`Is Valid`
      _)
    (:`Is Not Valid`
      (bind _returnvalue (`|CreateWidget` "/Game/UI/DeathScreen.DeathScreen_C" (`self.GetOwningPlayerController`)))
      (bind _output_get (set `self.DeathScreen` _returnvalue))))
  (`UserWidget.AddToViewport` _output_get 0)
  (`self.ShowCursor` _output_get))

(event `self.NotifyCharacterSpawned`
  (`self.CloseDeathScreen`)
  (`self.OpenHUD`))

(event `CloseDeathScreen`
  ;[1 1 1] Open/Close Death Screen
  (`Widget.RemoveFromParent` (`self.DeathScreen`)))

(event `OpenTeamMenu`
  ;[1 1 1] Open/Close Team Menu
  (`/Engine/EditorBlueprintResources/StandardMacros.IsValid` (`self.TeamScreen`)
    (:`Is Valid`
      _)
    (:`Is Not Valid`
      (bind _returnvalue (`|CreateWidget` "/Game/UI/TeamScreen.TeamScreen_C" (`self.GetOwningPlayerController`)))
      (bind _output_get (set `self.TeamScreen` _returnvalue))))
  (`UserWidget.AddToViewport` _output_get 0)
  (`self.ShowCursor` _output_get))

(event `CloseTeamMenu`
  ;[1 1 1] Open/Close Team Menu
  (`Widget.RemoveFromParent` (`self.TeamScreen`))
  (`self.HideCursor`))

(event `OpenClassMenu`
  ;[1 1 1] Open/Close Class Menu
  (`/Engine/EditorBlueprintResources/StandardMacros.IsValid` (`self.ClassMenu`)
    (:`Is Valid`
      _)
    (:`Is Not Valid`
      (bind _returnvalue (`|CreateWidget` "/Game/UI/ClassMenu.ClassMenu_C" (`self.GetOwningPlayerController`)))
      (bind _output_get (set `self.ClassMenu` _returnvalue))))
  (`UserWidget.AddToViewport` _output_get 0)
  (`self.ShowCursor` _output_get))

(event `CloseClassMenu`
  ;[1 1 1] Open/Close Class Menu
  (`Widget.RemoveFromParent` (`self.ClassMenu`))
  (`self.HideCursor`))

(event `OpenSpawnScreen`
  ;[1 1 1] Show/Hide Spawn Screen
  (`/Engine/EditorBlueprintResources/StandardMacros.IsValid` (`self.SpawnScreen`)
    (:`Is Valid`
      (`/Game/UI/TeamClassSpawnSelection/TeamClassAndSpawnPanel.Refresh Classes` (`self.SpawnScreen`)))
    (:`Is Not Valid`
      (bind _returnvalue (`|CreateWidget` "/Game/UI/TeamClassSpawnSelection/TeamClassAndSpawnPanel.TeamClassAndSpawnPanel_C" (`self.GetOwningPlayerController`)))
      (bind _output_get (set `self.SpawnScreen` _returnvalue))))
  (`UserWidget.AddToViewport` _output_get 0)
  (`self.ShowCursor` _output_get))

(event `CloseSpawnScreen`
  ;[1 1 1] Show/Hide Spawn Screen
  (`Widget.RemoveFromParent` (`self.SpawnScreen`))
  (`self.HideCursor`))

(fn `CreateDeathScreen`
  (bind _returnvalue (`self.GetOwningPlayerController`))
  (bind _returnvalue_2 (`|CreateWidget` "/Game/UI/DeathScreen.DeathScreen_C" _returnvalue))
  (set `self.DeathScreen` _returnvalue_2)
  (bind _asempires_player_controller (cast `EmpiresPlayerController` _returnvalue)
    (:`then`
      (set `/Game/UI/DeathScreen.LocalPlayerController` _asempires_player_controller (`self.DeathScreen`)))
    (:`CastFailed`
      _))
  (return))

(fn `HideDeathScreen`
  (if (not (`|EnumEquality` (`Widget.GetVisibility` (`self.DeathScreen`)) "Hidden"))
    (`Widget.RemoveFromParent` (`self.DeathScreen`)))
  (return))

(fn `ShowDeathScreen`
  (bind _deathscreen (`self.DeathScreen`))
  (`/Game/UI/DeathScreen.ListSpawnpoints` _deathscreen)
  (`UserWidget.AddToViewport` _deathscreen 0)
  (return))

(fn `UserConstructionScript`)