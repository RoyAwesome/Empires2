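; Game instance that runs the main menu flow and starts or joins multiplayer games.
; Menu and background widgets are created on first open, cached, then added to or removed from the viewport, with input switched between UI-only and game-only.
; Temporary host and join events run "open" console commands carrying the player name, then close the menu and restore game input.
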(event `EnterUIMode`
  (params (Focus :type "UserWidget Object Reference"))
  (bind _returnvalue (`GameplayStatics.GetPlayerController` 0))
  ;[1 1 1] Lock the mouse when needed
  (set `PlayerController.bShowMouseCursor` true _returnvalue)
  (`WidgetBlueprintLibrary.SetInputMode_UIOnlyEx` _returnvalue Focus true))

(event `ExitUIMode`
  (bind _returnvalue (`GameplayStatics.GetPlayerController` 0))
  ;[1 1 1] Lock the mouse when needed
  (set `PlayerController.bShowMouseCursor` false _returnvalue)
  (`WidgetBlueprintLibrary.SetInputMode_GameOnly` _returnvalue))

(event `OpenMainMenuLevel`
  ;[1 1 1] Open/Close the main menu level
  (`self.OpenMainMenuBackground`)
  (`self.OpenMainMenu`)
  (`self.EnterUIMode` (`self.MainMenu`)))

(event `LeaveMainMenuLevel`
  ;[1 1 1] Open/Close the main menu level
  (`self.CloseMainMenuBackground`)
  (`self.CloseMainMenu`)
  (`self.ExitUIMode`))

(event `OpenMainMenuBackground`
  ;[1 1 1] Open/Close Main Menu Background
  (`/Engine/EditorBlueprintResources/StandardMacros.IsValid` (`self.Background`)
    (:`Is Valid`
      _)
    (:`Is Not Valid`
      (bind _returnvalue (`|CreateWidget` "/Game/UI/MainMenu/Background.Background_C" (`GameplayStatics.GetPlayerController` 0)))
      (bind _output_get (set `self.Background` _returnvalue))))
  (`UserWidget.AddToViewport` _output_get 0))

(event `CloseMainMenuBackground`
  ;[1 1 1] Open/Close Main Menu Background
  (`Widget.RemoveFromParent` (`self.Background`)))

(event `ConnectToServer`
  (params (Host :type Text))
  ;[1 1 1] Temporary Host/Join server events
  (`KismetSystemLibrary.ExecuteConsoleCommand` (`KismetTextLibrary.Conv_TextToString` (`|FormatText` "open {ip}?name={playername}" Host (`self.PlayerName`))) (`GameplayStatics.GetPlayerController` 0))
  (`self.LeaveMainMenuLevel` :!label _label))

(event `OpenMainMenu`
  ;[1 1 1] Open/Close Main Menu
  (`/Engine/EditorBlueprintResources/StandardMacros.IsValid` (`self.MainMenu`)
    (:`Is Valid`
      _)
    (:`Is Not Valid`
      (bind _returnvalue (`|CreateWidget` "/Game/UI/MainMenu/MainMenu.MainMenu_C" (`GameplayStatics.GetPlayerController` 0)))
      (bind _output_get (set `self.MainMenu` _returnvalue))))
  (`UserWidget.AddToViewport` _output_get 0))

(event `HostServer`
  (params (Level :type Text))
  ;[1 1 1] Temporary Host/Join server events
  (`KismetSystemLibrary.ExecuteConsoleCommand` (`KismetTextLibrary.Conv_TextToString` (`|FormatText` "open {level}?listen?name={playername}" Level (`self.PlayerName`))) (`GameplayStatics.GetPlayerController` 0))
  (goto _label))

(event `CloseMainMenu`
  ;[1 1 1] Open/Close Main Menu
  (`Widget.RemoveFromParent` (`self.MainMenu`)))