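; Player controller for Empires that links the HUD's spawn screen to team, loadout and spawn point selection.
; The spawn screen opens on initial join or the OpenSpawnMenu input, and refreshes when the replicated CurrentTeam changes.
; Team requests go to EmpGamemode, loadouts to EmpPlayerState, and WantedSpawn is set directly or by matching EmpiresPlayerStart names as strings.
; Game messages print on screen tagged with their type.
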(event `self.ReceiveBeginPlay`)

(event `ClientGameMessage`
  (params (Message :type String) (MessageType :type "/Game/Blueprints/ClientMessageType Enum" :default "NewEnumerator0"))
  (`KismetSystemLibrary.PrintString` (`KismetTextLibrary.Conv_TextToString` (`|FormatText` "[{Type}] {Message}" (`KismetTextLibrary.Conv_StringToText` (`|GetEnumeratorNameAsString` MessageType)) (`KismetTextLibrary.Conv_StringToText` Message))) true true (struct :`G` 1.0 :`B` 0.110118 :`A` 1.0)))

(event `self.BPInitialGameJoin`
  ;[1 1 1] On the Initial Spawn, Show the Team Select Menu and the Class Select Menu
  (`self.ClientInitialJoin`))

(event `ClientInitialJoin`
  ;[1 1 1] On the Initial Spawn, Show the Team Select Menu and the Class Select Menu
  (bind _asemp_hud (cast `/Game/Blueprints/EmpHud` (`self.GetHUD`)))
  (`/Game/Blueprints/EmpHud.OpenSpawnScreen` _asemp_hud))

(event `RequestTeamChange`
  (params (TeamID :type Integer))
  ;[1 1 1] Team Change Events
  (bind _asemp_gamemode (cast `/Game/Blueprints/EmpGamemode` (`GameplayStatics.GetGameMode`)))
  (`/Game/Blueprints/EmpGamemode.RequestTeamChange` _asemp_gamemode self TeamID))

(event `RequestNewSpawnpoint`
  (params (SpawnPoint :type "EmpiresPlayerStart Object Reference"))
  (set `self.WantedSpawn` SpawnPoint))

(event `RequestSpectator`
  ;[1 1 1] Team Change Events
)

(event `Set Wanted Spawn Point`
  (params (WantedSpawnPoint :type String))
  (bind _outactors (`GameplayStatics.GetAllActorsOfClass` "/Script/Empires2.EmpiresPlayerStart"))
  (for _array_element _outactors
    (if (`KismetStringLibrary.EqualEqual_StrStr` (`KismetStringLibrary.Conv_ObjectToString` _array_element) WantedSpawnPoint)
      (set `self.WantedSpawn` _array_element))))

(event `InputAction|OpenSpawnMenu`
  (:`Pressed`
    (bind _asemp_hud (cast `/Game/Blueprints/EmpHud` (`self.GetHUD`)))
    (`/Game/Blueprints/EmpHud.OpenSpawnScreen` _asemp_hud)))

(event `RequestLoadoutChange`
  (params (Loadout :type "EmpInfantryClass.EmpClassLoadout Structure"))
  (bind _asemp_player_state (cast `/Game/Blueprints/EmpPlayerState` (`self.PlayerState`)))
  (set `EmpiresPlayerState.RequestedLoadout` Loadout _asemp_player_state))

(fn `OnRep_CurrentTeam`
  (bind _asemp_hud (cast `/Game/Blueprints/EmpHud` (`self.GetHUD`)))
  (`/Game/Blueprints/EmpHud.RefreshSpawnScreen` _asemp_hud))

(fn `UserConstructionScript`)