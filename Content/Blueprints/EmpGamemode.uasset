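; EmpGamemode handles player joins, team assignment, spawn selection and respawn checks.
; Joining players default to team 0; BeginPlay expires early-constructed characters and re-runs their initial join after a delay.
; Teams are copied to EmpGamestate for clients, since the game mode's array isn't replicated.
; Spawns use the controller's WantedSpawn, team changes skip capacity checks, and respawn checks team and class, messaging on failure.
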(event Custom|ReplicateTeams
  ;[1 1 1] The Teams array isn't replicated to clients in the gamemode, so give it to the GameState.
  (bind _asemp_gamestate (Utilities|Casting|CastToEmpGamestate (Game|GetGameState)))
  (for _array_element (Variables|Default|GetTeams)
    (Utilities|Array|Add (Variables|/Game/Blueprints/EmpGamestate.EmpGamestate_C|GetTeams _asemp_gamestate) _array_element)))

(event Custom|InitialPlayerStart
  (params (Controller :type Controller%20Object%20Reference))
  (bind _asemp_player_controller (Utilities|Casting|CastToEmpPlayerController Controller))
  (Variables|/Game/Blueprints/EmpPlayerController.EmpPlayerController_C|SetCurrentTeam _asemp_player_controller 0) ; TODO: Determine what team we should set him to
  (Class|EmpiresPlayerController|InitialGameJoin _asemp_player_controller))

(event EventBeginPlay
  (CallFunction|ReplicateTeams)
  ;[1 1 1] Local Server players are constructed before begin play (and before a gamemode can do anything with them.  Destroy them
  (bind _outactors (Actor|GetAllActorsOfClass "/Game/Blueprints/EmpCharacter.EmpCharacter_C"))
  (for _array_element _outactors
    (Actor|SetLifeSpan _array_element 0.1)
    (Utilities|FlowControl|Delay 1.0) ; Delay to give time for the teams to replicate
    (CallFunction|InitialPlayerStart (Pawn|GetController _array_element))))

(event EventBPPostLogin
  (params (NewPlayer :type Player%20Controller%20Object%20Reference))
  (bind _outactors (Actor|GetAllActorsOfClass "/Game/Blueprints/SpawnpointTypes/InitialSpectatorStartpoint.InitialSpectatorStartpoint_C"))
  (if (> (Utilities|Array|Length _outactors) 0)
    (Class|Controller|SetInitialLocationandRotation NewPlayer (.Location (Math|Transform|BreakTransform (Transformation|GetActorTransform (Utilities|Array|Get(acopy) _outactors (Math|Random|RandomIntegerinRange 0 (Utilities|Array|Length _outactors)))))) (.Rotation (Math|Transform|BreakTransform (Transformation|GetActorTransform (Utilities|Array|Get(acopy) _outactors (Math|Random|RandomIntegerinRange 0 (Utilities|Array|Length _outactors)))))))))

(event EventPostLogin
  (params (NewPlayer :type Player%20Controller%20Object%20Reference))
  (CallFunction|InitialPlayerStart NewPlayer))

(fn ConstructionScript)

(fn BPChoosePlayerStart
  (params (Player :type Controller%20Object%20Reference))
  (bind _asemp_player_controller (Utilities|Casting|CastToEmpPlayerController Player))
  (Utilities|IsValid 0
    (:Is%20Valid
      (return (Variables|/Script/Empires2.EmpiresPlayerController|GetWantedSpawn _asemp_player_controller)))))

(fn RequestTeamChange
  (params (Player :type Controller%20Object%20Reference) (RequestedTeam :type Integer :default 0))
  (bind _asemp_player_controller (Utilities|Casting|CastToEmpPlayerController Player))
  (Variables|/Game/Blueprints/EmpPlayerController.EmpPlayerController_C|SetCurrentTeam _asemp_player_controller RequestedTeam)
  (return true) ; TODO: Check to see if the team can hold this player
)

(fn CanRespawnPlayer
  (params (Controller :type Player%20Controller%20Object%20Reference))
  (bind _asemp_player_controller (Utilities|Casting|CastToEmpPlayerController Controller))
  ;[1 1 1] Determine if we have a correct Team
  (if (and (>= (Variables|/Game/Blueprints/EmpPlayerController.EmpPlayerController_C|GetCurrentTeam _asemp_player_controller) 0) (< (Variables|/Game/Blueprints/EmpPlayerController.EmpPlayerController_C|GetCurrentTeam _asemp_player_controller) (Utilities|Array|Length (Variables|Default|GetTeams))))
    (LocalVariables|SetRet true)
    ;[1 1 1] Determine if we have a correct Class
    (if (and (< (Utilities|Array|Length (Variables|/Script/Empires2.EmpTeam|GetClasses (.Faction (Utilities|Struct|BreakTeamDefinition (Utilities|Array|Get(acopy) (Variables|Default|GetTeams) (Variables|/Game/Blueprints/EmpPlayerController.EmpPlayerController_C|GetCurrentTeam _asemp_player_controller)))))) (Variables|/Game/Blueprints/EmpPlayerController.EmpPlayerController_C|GetWantedClass _asemp_player_controller)) (>= (Variables|/Game/Blueprints/EmpPlayerController.EmpPlayerController_C|GetWantedClass _asemp_player_controller) 0))
      ;[1 1 1] Respawn Succeeded
      (LocalVariables|SetRet true)
      (else
        (Default|ClientGameMessage _asemp_player_controller "Cannot Respawn: Class Invalid" "NewEnumerator1")
        ;[1 1 1] Failed to Respawn
        (LocalVariables|SetRet false :!label _label)))
    (else
      (Default|ClientGameMessage _asemp_player_controller "Cannot Respawn: Team Not Selected" "NewEnumerator1")
      (goto _label)))
  (return (LocalVariables|GetRet)))