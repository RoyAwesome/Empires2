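; TestHUD is a HUD Blueprint that manages the death screen and ammo counter widgets for the local player.
; BeginPlay creates both widgets and hands the death screen the EmpiresPlayerController.
; Death shows the death screen with its spawnpoint list, while spawning hides it, binds the possessed Empires2Character to the ammo counter and displays it.
; Damage and landed-hit notifications only print debug strings.
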(event `self.ReceiveBeginPlay`
  ;[1 1 1] When the Hud starts, Create the widgets we need
  (`self.CreateDeathScreen`)
  (`self.CreateHUDElements`))

(event `self.NotifyDied`
  (params (Killer :type "PlayerState Object Reference"))
  (`self.ShowDeathScreen`))

(event `self.NotifyTookDamage`
  (params (FromWhere :type "Object.Vector Structure") (HowMuch :type Integer) (FromWho :type "PlayerState Object Reference"))
  (`KismetSystemLibrary.PrintString` "Took Damage"))

(event `self.NotifyCharacterSpawned`
  (`self.HideDeathScreen`)
  (`self.SetCreatedPawn`)
  (`self.ShowHudElements`))

(event `self.NotifyLandedHit`
  (params (HitWhat :type "Pawn Object Reference"))
  (`KismetSystemLibrary.PrintString` "Hit Someone"))

(fn `CreateDeathScreen`
  (bind _returnvalue (`self.GetOwningPlayerController`))
  (bind _returnvalue_2 (`|CreateWidget` "/Game/UI/DeathScreen.DeathScreen_C" _returnvalue))
  (set `self.DeathScreen` _returnvalue_2)
  (bind _asempiresplayercontroller (cast `EmpiresPlayerController` _returnvalue)
    (:`then`
      (set `/Game/UI/DeathScreen.LocalPlayerController` _asempiresplayercontroller (`self.DeathScreen`)))
    (:`CastFailed`
      _))
  (return))

(fn `CreateHUDElements`
  (bind _returnvalue (`|CreateWidget` "/Game/UI/AmmoCounter.AmmoCounter_C" (`self.GetOwningPlayerController`)))
  (set `self.Hud` _returnvalue)
  (return))

(fn `HideDeathScreen`
  (bind _returnvalue (`Widget.GetVisibility` (`self.DeathScreen`)))
  (if (not (`|EnumEquality` _returnvalue "Hidden"))
    (`UserWidget.RemoveFromViewport` (`self.DeathScreen`)))
  (return))

(fn `HideHUDElements`
  (bind _returnvalue (`Widget.GetVisibility` (`self.Hud`)))
  (if (not (`|EnumEquality` _returnvalue "Hidden"))
    (`UserWidget.RemoveFromViewport` (`self.Hud`))))

(fn `SetCreatedPawn`
  (bind _asempires2character (cast `Empires2Character` (`Controller.K2_GetPawn` (`self.GetOwningPlayerController`))))
  (set `/Game/UI/AmmoCounter.Character` _asempires2character (`self.Hud`)))

(fn `ShowDeathScreen`
  (bind _deathscreen (`self.DeathScreen`))
  (`/Game/UI/DeathScreen.ListSpawnpoints` _deathscreen)
  (`UserWidget.AddToViewport` _deathscreen)
  (return))

(fn `ShowHudElements`
  (`UserWidget.AddToViewport` (`self.Hud`)))

(fn `UserConstructionScript`)